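; BP_DevDoor is a development door that moves the game to a target map when the host player walks into it.
; Box overlap by a PRPlayerCharacter triggers PRGameInstance ServerTravelToMap, but only with authority and when that character's controller is player controller 0.
; A widget component shows the MapName through W_WorldText, set in both the construction script and BeginPlay.
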(event `self.Box.OnComponentBeginOverlap`
  (params (OverlappedComponent :type "PrimitiveComponent Object Reference") (OtherActor :type "Actor Object Reference") (OtherComp :type "PrimitiveComponent Object Reference") (OtherBodyIndex :type Integer) (bFromSweep :type Boolean) (SweepResult :type "HitResult Structure (by ref)"))
  (bind _asprplayer_character (cast `PRPlayerCharacter` OtherActor))
  (bind _asprplayer_controller (cast `PRPlayerController` (`Pawn.GetController` _asprplayer_character)))
  (if (`self.HasAuthority` _asprplayer_controller)
    (if (== (`GameplayStatics.GetPlayerController` 0) _asprplayer_controller)
      (bind _asprgame_instance (cast `PRGameInstance` (`GameplayStatics.GetGameInstance`)))
      (`PRGameInstance.ServerTravelToMap` _asprgame_instance (`self.TargetMap`) false))))

(event `self.ReceiveBeginPlay`
  (bind _asw_door_text (cast `/Game/4_Dev/Door/W_WorldText` (`WidgetComponent.GetWidget` (`self.Widget`))))
  (`/Game/4_Dev/Door/W_WorldText.SetText` _asw_door_text (`self.MapName`)))

(fn `UserConstructionScript`
  (bind _asw_door_text (cast `/Game/4_Dev/Door/W_WorldText` (`WidgetComponent.GetWidget` (`self.Widget`))))
  (`/Game/4_Dev/Door/W_WorldText.SetText` _asw_door_text (`self.MapName`)))