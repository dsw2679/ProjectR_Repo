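; BP_MovingWall is a test prop, a wall that slides back and forth along the world Y axis around its starting location.
; BeginPlay stores the origin, and Tick advances a time accumulator that drives a sine offset from that origin.
; Only the instance with authority sets the actor location, though every instance advances the accumulator.
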(event `self.ReceiveBeginPlay`
  (set `self.OriginLocation` (`self.K2_GetActorLocation`)))

(event `self.ReceiveTick`
  (params (DeltaSeconds :type "Float (single-precision)"))
  (set `self.Aggregator` (+ (`self.Aggregator`) (* DeltaSeconds 0.4)))
  (if (`self.HasAuthority`)
    (`self.K2_SetActorLocation` (`KismetMathLibrary.MakeVector` (.x (`self.OriginLocation`)) (+ (.y (`self.OriginLocation`)) (* (`KismetMathLibrary.Sin` (`self.Aggregator`)) 600.0)) (.z (`self.OriginLocation`))))))

(fn `UserConstructionScript`)