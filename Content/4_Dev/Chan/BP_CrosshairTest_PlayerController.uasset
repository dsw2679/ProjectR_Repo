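; Test player controller for trying out crosshair feedback on BP_CrosshairTest_HUD.
; Key 1 casts the current HUD and triggers its hit reaction.
; Key 2 casts the same HUD and triggers a recoil effect with fixed speed and strength.
; BeginPlay, Tick and the construction script add no logic of their own.
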(event `Key|One`
  (params (Key :type "Key Structure"))
  (:`Pressed`
    (bind _asbp_test_gameplay_hud (cast `/Game/4_Dev/Chan/BP_CrosshairTest_HUD` (`self.GetHUD`)))
    (`/Game/4_Dev/Chan/BP_CrosshairTest_HUD.OnHit` _asbp_test_gameplay_hud)))

(event `Key|Two`
  (params (Key :type "Key Structure"))
  (:`Pressed`
    (bind _asbp_test_gameplay_hud (cast `/Game/4_Dev/Chan/BP_CrosshairTest_HUD` (`self.GetHUD`)))
    (`/Game/4_Dev/Chan/BP_CrosshairTest_HUD.OnRecoil` _asbp_test_gameplay_hud 4.0 8.0)))

(fn `UserConstructionScript`
  (`parent.UserConstructionScript`))