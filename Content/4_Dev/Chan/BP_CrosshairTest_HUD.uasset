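; Test HUD Blueprint that displays a configurable crosshair and passes combat feedback to it.
; On BeginPlay it creates W_CrosshairTestHUD, adds it to the viewport, caches its crosshair widget and initializes it with the cross-style DA_CrosshairConfig_Cross data asset.
; OnHit and OnRecoil events forward hit feedback and recoil speed and strength to that widget after a validity check.
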(event `self.ReceiveBeginPlay`
  (bind _returnvalue (`|CreateWidget` "/Game/4_Dev/Chan/W_CrosshairTestHUD.W_CrosshairTestHUD_C"))
  (bind _output_get (set `self.HUD` _returnvalue))
  (`UserWidget.AddToViewport` _output_get 0)
  (bind _wb_crosshair_h (`/Game/4_Dev/Chan/W_CrosshairTestHUD.GetCrosshairWidget` (`self.HUD`)))
  (bind _output_get_2 (set `self.Crosshair` _wb_crosshair_h))
  (`PRCrosshairInterface.InitCrosshair` _output_get_2 "/Game/0_BP/Data/Crosshair/DA_CrosshairConfig_Cross.DA_CrosshairConfig_Cross"))

(event `OnHit`
  (bind _crosshair (`self.Crosshair`)
    (:`then`
      (`/Game/0_BP/UI/Crosshair/W_Crosshair.OnHit` _crosshair))
    (:`else`)))

(event `OnRecoil`
  (params (Speed :type "Float (single-precision)") (Strength :type "Float (single-precision)"))
  (bind _crosshair (`self.Crosshair`)
    (:`then`
      (`/Game/0_BP/UI/Crosshair/W_Crosshair.OnRecoil` _crosshair Speed Strength))
    (:`else`)))

(fn `UserConstructionScript`)