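; Gameplay ability that handles the reviving character's animation flow during a revive.
; On either direct or event-triggered activation, it sets the avatar's weapon to unarmed, plays the revive montage and listens for Finished and Canceled gameplay events.
; Each event plays its closing montage, which is allowed to outlive the ability, then any montage exit ends the ability with a debug print.
; It applies no revive effect itself.
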(event `self.K2_ActivateAbility`
  (`|ExecutionSequence` :!label _label
    (:`then_0`
      (bind _returnvalue (`PRGameplayStatics.GetWeaponManagerComponent` (`self.GetAvatarActorFromActorInfo`)))
      (`/Engine/EditorBlueprintResources/StandardMacros.IsValid` _returnvalue
        (:`Is Valid`
          (`PRWeaponManagerComponent.SetWeaponArmedState` _returnvalue "Unarmed"))))
    (:`then_1`
      (`AbilityTask_PlayMontageAndWait.CreatePlayMontageAndWaitProxy` "None" "/Game/2_Characters/RCharacter/Animation/AnimMontage/AM_Player_M_UN_Action_Revive.AM_Player_M_UN_Action_Revive"
        (:`then`
          (`AbilityTask_WaitGameplayEvent.WaitGameplayEvent` (struct :`TagName` "Event.Ability.Revive.Finished") null
            (:`then`
              (`AbilityTask_WaitGameplayEvent.WaitGameplayEvent` (struct :`TagName` "Event.Ability.Revive.Canceled") null
                (:`EventReceived`
                  (`AbilityTask_PlayMontageAndWait.CreatePlayMontageAndWaitProxy` "None" "/Game/2_Characters/RCharacter/Animation/AnimMontage/AM_Player_M_UN_Action_Revive_Cancel.AM_Player_M_UN_Action_Revive_Cancel" 1.0 "None" false 1.0 0.0 true
                    (:`OnCompleted`
                      _)
                    (:`OnBlendOut`
                      _)
                    (:`OnInterrupted`
                      _)
                    (:`OnCancelled`
                      _))
                  (`self.K2_EndAbility`)
                  (`KismetSystemLibrary.PrintString` "Revive Canceled"))))
            (:`EventReceived`
              (`AbilityTask_PlayMontageAndWait.CreatePlayMontageAndWaitProxy` "None" "/Game/2_Characters/RCharacter/Animation/AnimMontage/AM_Player_M_UN_Action_Revive_End.AM_Player_M_UN_Action_Revive_End" 1.0 "None" false 1.0 0.0 true
                (:`OnCompleted`
                  _)
                (:`OnBlendOut`
                  _)
                (:`OnInterrupted`
                  _)
                (:`OnCancelled`
                  _))
              (`self.K2_EndAbility`)
              (`KismetSystemLibrary.PrintString` "Revive Finished"))))))))

(event `self.K2_ActivateAbilityFromEvent`
  (params (EventData :type "GameplayEventData Structure (by ref)"))
  (goto _label))

(event `self.K2_OnEndAbility`
  (params (bWasCancelled :type Boolean))
  (`KismetSystemLibrary.PrintString` "Endability"))