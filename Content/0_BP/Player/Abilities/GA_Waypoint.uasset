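; Player gameplay ability that plays the grab and release animations for a waypoint action.
; On activation, directly or from an event, it sets the avatar's weapon manager to Unarmed and starts the grab montage.
; It then waits for the Waypoint End gameplay event, plays the release montage and ends when that finishes or is cut short.
; Ending the ability also cancels abilities tagged as player interaction.
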(event `self.K2_ActivateAbilityFromEvent`
  (params (EventData :type "GameplayEventData Structure (by ref)"))
  (`|ExecutionSequence` :!label _label
    (:`then_0`
      (bind _returnvalue (`PRGameplayStatics.GetWeaponManagerComponent` (`self.GetAvatarActorFromActorInfo`)))
      (`/Engine/EditorBlueprintResources/StandardMacros.IsValid` _returnvalue
        (:`Is Valid`
          (`PRWeaponManagerComponent.SetWeaponArmedState` _returnvalue "Unarmed"))))
    (:`then_1`
      (`AbilityTask_PlayMontageAndWait.CreatePlayMontageAndWaitProxy` "None" "/Game/2_Characters/RCharacter/Animation/AnimMontage/AM_Player_M_UN_Action_Waypoint_Grab.AM_Player_M_UN_Action_Waypoint_Grab"
        (:`then`
          (`AbilityTask_WaitGameplayEvent.WaitGameplayEvent` (struct :`TagName` "Event.Ability.Waypoint.End") null
            (:`EventReceived`
              (`AbilityTask_PlayMontageAndWait.CreatePlayMontageAndWaitProxy` "None" "/Game/2_Characters/RCharacter/Animation/AnimMontage/AM_Player_M_UN_Action_Waypoint_Release.AM_Player_M_UN_Action_Waypoint_Release"
                (:`OnCompleted`
                  _)
                (:`OnBlendOut`
                  _)
                (:`OnInterrupted`
                  _)
                (:`OnCancelled`
                  _))
              (`self.K2_EndAbility`))))))))

(event `self.K2_ActivateAbility`
  (goto _label))

(event `self.K2_OnEndAbility`
  (params (bWasCancelled :type Boolean))
  (`PRGameplayStatics.CancelAbilityWithTags` null (`BlueprintGameplayTagLibrary.MakeGameplayTagContainerFromTag` (struct :`TagName` "Ability.Player.Interaction"))))