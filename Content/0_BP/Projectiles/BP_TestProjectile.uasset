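; BP_TestProjectile is a test projectile that leaves a healing area where it is destroyed.
; BeginPlay gives it a five-second lifespan.
; On destruction, only the authority spawns a BP_HealArea at the projectile's transform.
; It initializes that area with the projectile's gameplay effect spec and instigator ability system component for a short fixed duration.
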(event `self.ReceiveBeginPlay`
  (`self.SetLifeSpan` 5.0))

(event `self.OnProjectileDestroyed`
  (if (`self.HasProjectileAuthority`)
    (bind _returnvalue (`|SpawnActorFromClass` "/Game/0_BP/World/Area/BP_HealArea.BP_HealArea_C" (`KismetMathLibrary.MakeTransform` (`self.K2_GetActorLocation`) (`self.K2_GetActorRotation`)) "Undefined" "MultiplyWithRoot" null null))
    (`/Engine/EditorBlueprintResources/StandardMacros.IsValid` _returnvalue
      (:`Is Valid`
        (`PREffectArea.InitEffectArea` _returnvalue (`self.EffectSpecHandle`) (`self.InstigatorASC`) 3.0)))))

(fn `UserConstructionScript`)