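; BP_Interaction_Revive is an interaction that lets a downed owner be revived.
; CanInteract allows it only when the owner's Ability System Component has the State.Down gameplay tag, regardless of the interactor.
; Execute sends the Event.Ability.GetUp gameplay event to that component's owning actor, leaving the get-up logic to whatever handles the event.
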(event `self.Execute`
  (params (Interactor :type "Actor Object Reference"))
  (bind _returnvalue (`PRGameplayStatics.GetAbilitySystemComponent` (`self.GetOwner`)))
  (`/Engine/EditorBlueprintResources/StandardMacros.IsValid` _returnvalue
    (:`Is Valid`
      (`AbilitySystemBlueprintLibrary.SendGameplayEventToActor` (`ActorComponent.GetOwner` _returnvalue) (struct :`TagName` "Event.Ability.GetUp")))))

(fn `CanInteract`
  (params (Interactor :type "Actor Object Reference"))
  (returns (ReturnValue :type Boolean))
  (bind _returnvalue (`PRGameplayStatics.GetAbilitySystemComponent` (`self.GetOwner`)))
  (`/Engine/EditorBlueprintResources/StandardMacros.IsValid` _returnvalue
    (:`Is Valid`
      (return (`GameplayTagAssetInterface.HasMatchingGameplayTag` _returnvalue (struct :`TagName` "State.Down"))))
    (:`Is Not Valid`
      (return false))))