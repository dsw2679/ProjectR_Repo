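; BP_FogWall is a configurable fog wall actor with gate mesh, wall mesh, Niagara smoke and point light, switched by EnableWall and DisableWall.
; The construction script applies exposed meshes, colors, light and smoke settings, creating dynamic materials for wall and smoke.
; Enabling sets query-and-physics collision, starts smoke and plays a timeline fading in wall opacity and light intensity.
; Disabling reverts to query-only collision, stops smoke and reverses the timeline.
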(event `EnableWall`
  ;[0 0 0] Enable/Disable
  (`PrimitiveComponent.SetCollisionEnabled` (`self.SM_FogWall`) "QueryAndPhysics")
  (`ActorComponent.Activate` (`self.NS_Smoke`) false)
  (bind (_direction _value) (`Timeline|Lerp` :!via `PlayFromStart` :!label _label)
    (:`Update`
      (`MaterialInstanceDynamic.SetScalarParameterValue` (`self.DynamicFogWallMaterial`) "Opacity" _value)
      (`LightComponent.SetIntensity` (`self.PointLight`) (* _value (`self.LightIntensity`))))))

(event `DisableWall`
  ;[0 0 0] Enable/Disable
  (`PrimitiveComponent.SetCollisionEnabled` (`self.SM_FogWall`) "QueryOnly")
  (`ActorComponent.Deactivate` (`self.NS_Smoke`))
  (goto _label :!via `ReverseFromEnd`))

(fn `LerpValue`)

(fn `UserConstructionScript`
  ;[0 0 0] Light
  (`LightComponent.SetIntensity` (`self.PointLight`) (`self.LightIntensity`))
  (`LightComponent.SetLightColor` (`self.PointLight`) (`self.LightColor`) true)
  (`LocalLightComponent.SetAttenuationRadius` (`self.PointLight`) (`self.LightAttenuationRadius`))
  ;[0 0 0] Dynamic Materials
  (bind _returnvalue (`PrimitiveComponent.CreateDynamicMaterialInstance` (`self.SM_FogWall`) 0 (`self.FogWallMaterial`) "None"))
  (set `self.DynamicFogWallMaterial` _returnvalue)
  (bind _returnvalue_2 (`KismetMaterialLibrary.CreateDynamicMaterialInstance` (`self.SmokeMaterial`)))
  (set `self.DynamicSmokeMaterial` _returnvalue_2)
  ;[0 0 0] Meshes
  (`StaticMeshComponent.SetStaticMesh` (`self.SM_Gate`) (`self.GateMesh`))
  (`StaticMeshComponent.SetStaticMesh` (`self.SM_FogWall`) (`self.WallMesh`))
  ;[0 0 0] Smoke
  (`NiagaraComponent.SetVariableMaterial` (`self.NS_Smoke`) "SmokeMaterial" (`self.DynamicSmokeMaterial`))
  (`FXSystemComponent.SetFloatParameter` (`self.NS_Smoke`) "SmokeSpawnWidth" (`self.SmokeSpawnAreaWidth`))
  (`FXSystemComponent.SetFloatParameter` (`self.NS_Smoke`) "SmokeSpawnCount" (`self.SmokeSpawnCount`))
  (`FXSystemComponent.SetFloatParameter` (`self.NS_Smoke`) "SmokeSize" (`self.SmokeSize`))
  (`MaterialInstanceDynamic.SetVectorParameterValue` (`self.DynamicSmokeMaterial`) "Color" (`self.SmokeColor`))
  ;[0 0 0] Wall Colors
  (`MaterialInstanceDynamic.SetVectorParameterValue` (`self.DynamicFogWallMaterial`) "Color" (`self.WallColor`))
  (`MaterialInstanceDynamic.SetVectorParameterValue` (`self.DynamicFogWallMaterial`) "Color_Energy" (`self.WallEnergyColor`)))